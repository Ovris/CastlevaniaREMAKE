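; BP_Whip is the whip weapon actor, which damages enemies caught in its capsule when an attack begins.
; The begin-attack event enables query-only collision and sends TakeDamageMessage with DMG and the player character to each overlapping actor tagged Enemy, printing debug text.
; The end-attack event disables collision.
; Hits come from that single overlap check, as the overlap event handlers are empty.
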(event `self.Capsule.OnComponentBeginOverlap`
  (params (OverlappedComponent :type "PrimitiveComponent Object Reference") (OtherActor :type "Actor Object Reference") (OtherComp :type "PrimitiveComponent Object Reference") (OtherBodyIndex :type Integer) (bFromSweep :type Boolean) (SweepResult :type "HitResult Structure (by ref)")))

(event `self.ReceiveActorBeginOverlap`
  (params (OtherActor :type "Actor Object Reference")))

(event `/Game/CastlevaniaREMAKE/Yana/BPI_AttackHandler.BeginAttack_SetWhipCollisionON`
  (bind _capsule (`self.Capsule`))
  (`PrimitiveComponent.SetCollisionEnabled` _capsule "QueryOnly")
  (for _array_element (`PrimitiveComponent.GetOverlappingActors` _capsule "/Script/Engine.Actor")
    (if (`self.ActorHasTag` _array_element "Enemy")
      (`KismetSystemLibrary.PrintString` "Hello" true true (struct :`R` 0.128474 :`G` 1.0 :`A` 1.0))
      (message `/Game/CastlevaniaREMAKE/Yana/BPI_AttackHandler.TakeDamage` _array_element (`self.DMG`) (`GameplayStatics.GetPlayerCharacter` 0)))))

(event `/Game/CastlevaniaREMAKE/Yana/BPI_AttackHandler.EndAttack_SetWhipCollisionOFF`
  (`PrimitiveComponent.SetCollisionEnabled` (`self.Capsule`) "NoCollision"))

(fn `UserConstructionScript`)